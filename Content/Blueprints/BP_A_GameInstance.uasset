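; Game instance Blueprint that owns background music for the front end and gameplay.
; Each track has play and stop events, with the audio component created lazily as a 2D sound that persists across level transitions and is cached for reuse.
; Play starts a track only if it is not already playing, and stop fades out a playing track briefly.
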(event `PlayFrontEndBGM`
  (`/Engine/EditorBlueprintResources/StandardMacros.IsValid` (`self.FrontEndAudio`)
    (:`Is Valid`
      (if (not (`AudioComponent.IsPlaying` (`self.FrontEndAudio`)))
        (`AudioComponent.Play` (`self.FrontEndAudio`) 0.0)))
    (:`Is Not Valid`
      (bind _returnvalue (`GameplayStatics.CreateSound2D` "/Game/Assets/Audio/BGM_FrontEnd.BGM_FrontEnd" 1.0 1.0 0.0 null true))
      (bind _output_get (set `self.FrontEndAudio` _returnvalue))
      (`AudioComponent.Play` _output_get 0.0))))

(event `StopFrontEndBGM`
  (`/Engine/EditorBlueprintResources/StandardMacros.IsValid` (`self.FrontEndAudio`)
    (:`Is Valid`
      (if (`AudioComponent.IsPlaying` (`self.FrontEndAudio`))
        (`AudioComponent.FadeOut` (`self.FrontEndAudio`) 0.5 0.0 "Linear")))))

(event `PlayGameplayBGM`
  (`/Engine/EditorBlueprintResources/StandardMacros.IsValid` (`self.GameplayAudio`)
    (:`Is Valid`
      (if (not (`AudioComponent.IsPlaying` (`self.GameplayAudio`)))
        (`AudioComponent.Play` (`self.GameplayAudio`) 0.0)))
    (:`Is Not Valid`
      (bind _returnvalue (`GameplayStatics.CreateSound2D` "/Game/Assets/Audio/BGM_Gameplay.BGM_Gameplay" 1.0 1.0 0.0 null true))
      (bind _output_get (set `self.GameplayAudio` _returnvalue))
      (`AudioComponent.Play` _output_get 0.0))))

(event `StopGameplayBGM`
  (`/Engine/EditorBlueprintResources/StandardMacros.IsValid` (`self.GameplayAudio`)
    (:`Is Valid`
      (if (`AudioComponent.IsPlaying` (`self.GameplayAudio`))
        (`AudioComponent.FadeOut` (`self.GameplayAudio`) 0.5 0.0 "Linear")))))