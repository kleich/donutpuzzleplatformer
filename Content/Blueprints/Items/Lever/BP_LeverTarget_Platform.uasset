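; A lever target platform that moves its mesh along a spline when its attached lever is flipped.
; On BeginPlay it registers an event with the lever's flipped delegate, and a FlipFlop alternates each flip between playing and reversing a timeline.
; The timeline's Distance track scales the spline length to set the mesh's world location, without sweeping.
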(event `self.ReceiveBeginPlay`
  (add `/Game/Blueprints/Items/Lever/BP_Lever.LeverFlippedDelegate` (`self.AttachedLever`) (delegate `LeverFlippedDelegate_Event_0`)))

(event `LeverFlippedDelegate_Event_0`
  (`/Engine/EditorBlueprintResources/StandardMacros.FlipFlop`
    (:`A`
      (bind (_direction _distance) (`Timeline|Timeline_0` :!label _label)
        (:`Update`
          (`SceneComponent.K2_SetWorldLocation` (`self.StaticMesh`) (`SplineComponent.GetLocationAtDistanceAlongSpline` (`self.Spline`) (* _distance (`SplineComponent.GetSplineLength` (`self.Spline`))) "World") false false))))
    (:`B`
      (goto _label :!via `Reverse`))))

(fn `UserConstructionScript`)