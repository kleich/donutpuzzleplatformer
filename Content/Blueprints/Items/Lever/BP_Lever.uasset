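; BP_Lever is an interactable lever that responds to the player character's pickup event while it is interactable.
; A FlipFlop alternately plays and reverses a timeline that rotates the mesh, with interaction and prompt text disabled during the swing.
; When the timeline finishes, it restores interaction and fires LeverFlippedDelegate.
; Its own handler then disables single-use levers permanently or toggles LeverFlipped again on reusable ones.
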(event `self.ReceiveBeginPlay`
  ;[1 1 1] Set player ref + bind to pickup delegate
  (`parent.ReceiveBeginPlay`)
  (bind _asbp_player_character (cast `/Game/Blueprints/PlayerCharacter/BP_PlayerCharacter` (`GameplayStatics.GetPlayerPawn` 0)))
  (bind _output_get (set `self.PlayerRef` _asbp_player_character))
  (add `/Game/Blueprints/PlayerCharacter/BP_PlayerCharacter.Pickup_Event` _output_get (delegate `Pickup_Sequence`))
  (add `self.LeverFlippedDelegate` (delegate `Lever_FlippedEvent`)))

(event `Lever_FlippedEvent`
  (if (`self.bSingleUse`)
    (set `self.bInteractable` false)
    (`SceneComponent.SetVisibility` (`self.InteractText`) false false)
    (set `PrimitiveComponent.bGenerateOverlapEvents` false (`self.InteractOverlapArea`))
    (else
      (set `self.bLeverFlipped` (not (`self.bLeverFlipped`))))))

(event `Pickup_Sequence`
  ;[1 1 1] Pickup Sequence Event
  (if (`self.bInteractable`)
    (set `self.bInteractable` false)
    (`SceneComponent.SetVisibility` (`self.InteractText`) false false)
    (`/Engine/EditorBlueprintResources/StandardMacros.FlipFlop`
      (:`A`
        (set `self.bLeverFlipped` true)
        (bind (_direction _rotation) (`Timeline|RotateLever` :!via `PlayFromStart` :!label _label)
          (:`Update`
            (`SceneComponent.K2_SetRelativeRotation` (`self.Mesh`) (`KismetMathLibrary.MakeRotator` 0.0 _rotation 90.0) false false))
          (:`Finished`
            (set `self.bInteractable` true)
            (`SceneComponent.SetVisibility` (`self.InteractText`) true false)
            (`self.LeverFlippedDelegate`))))
      (:`B`
        (set `self.bLeverFlipped` false)
        (goto _label :!via `Reverse`)))))

(fn `UserConstructionScript`
  (`parent.UserConstructionScript`))