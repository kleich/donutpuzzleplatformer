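; Interactable door that the player opens when holding at least one key, reporting a fixed score value to the player's door stats.
; It binds to the player character's pickup event at BeginPlay and responds only while flagged interactable.
; Opening hides the prompt text, turns off overlap events on the interact area and plays a timeline that drives the door's yaw.
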(event `self.ReceiveBeginPlay`
  ;[1 1 1] Set player ref + bind to pickup delegate
  (`parent.ReceiveBeginPlay`)
  (bind _asbp_player_character (cast `/Game/Blueprints/PlayerCharacter/BP_PlayerCharacter` (`A_BlueprintFunctionLibrary.GetActivePlayerCharacter`)))
  (bind _output_get (set `self.PlayerRef` _asbp_player_character))
  (add `/Game/Blueprints/PlayerCharacter/BP_PlayerCharacter.Pickup_Event` _output_get (delegate `Pickup_Sequence`)))

(event `Pickup_Sequence`
  ;[1 1 1] Pickup Sequence Event
  (if (`self.bInteractable`)
    (if (> (`/Game/Blueprints/PlayerCharacter/BP_PlayerCharacter.NumKeys` (`self.PlayerRef`)) 0)
      (`/Game/Blueprints/PlayerCharacter/BP_PlayerCharacter.SetDoorCountStats` (`self.PlayerRef`) (`self.ScoreVale`))
      (`SceneComponent.SetVisibility` (`self.InteractText`) false false)
      (set `PrimitiveComponent.bGenerateOverlapEvents` false (`self.InteractOverlapArea`))
      (bind (_direction _rotation) (`Timeline|OpenDoor`)
        (:`Update`
          (`SceneComponent.K2_SetRelativeRotation` (`self.door`) (`KismetMathLibrary.MakeRotator` 0.0 0.0 _rotation) false false))))))

(fn `UserConstructionScript`
  (`parent.UserConstructionScript`)
  (set `self.ScoreVale` 125))