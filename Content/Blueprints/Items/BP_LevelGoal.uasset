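; BP_LevelGoal is a level goal actor that awards achievements when the player character overlaps it.
; It unlocks NoDeaths if the player is still eligible, then picks a completion achievement by comparing the current level name as text.
; Any level other than A1_Level or A1_LevelTwo counts as the third.
; After a short delay it sets the GoalReached flag, with nothing in this file reading it.
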(event `self.ReceiveActorBeginOverlap`
  (params (OtherActor :type "Actor Object Reference"))
  (bind _asbp_player_character (cast `/Game/Blueprints/PlayerCharacter/BP_PlayerCharacter` OtherActor))
  (if (`/Game/Blueprints/PlayerCharacter/BP_PlayerCharacter.EligibleForNoDeathsAchievement` _asbp_player_character)
    ;[1 1 1] Unlock "No Deaths" Achievement if eligible (did not die during level)
    (`AchievementSubSystem.Unlock` (`A_BlueprintFunctionLibrary.GetAchievementSystem`) "NoDeaths"))
  (bind _returnvalue (`GameplayStatics.GetCurrentLevelName` true))
  (bind _returnvalue_2 (`KismetTextLibrary.Conv_StringToText` _returnvalue))
  (if (`KismetTextLibrary.EqualEqual_TextText` _returnvalue_2 "A1_Level")
    (`AchievementSubSystem.Unlock` (`A_BlueprintFunctionLibrary.GetAchievementSystem`) "LevelComplete1")
    (elif (`KismetTextLibrary.EqualEqual_TextText` _returnvalue_2 "A1_LevelTwo")
      (`AchievementSubSystem.Unlock` (`A_BlueprintFunctionLibrary.GetAchievementSystem`) "LevelComplete2")
      (else
        (`AchievementSubSystem.Unlock` (`A_BlueprintFunctionLibrary.GetAchievementSystem`) "LevelComplete3"))))
  (`KismetSystemLibrary.Delay` 2.0)
  (set `self.bGoalReached` true))

(fn `UserConstructionScript`)