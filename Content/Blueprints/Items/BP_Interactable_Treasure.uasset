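; BP_Interactable_Treasure is a treasure pickup that adds its score to the player's treasure count.
; On BeginPlay it runs the parent logic, stores the active player character and binds to that player's pickup event.
; When the event fires while the treasure is interactable, it passes its score, set in the construction script, to the player's treasure stats and destroys itself.
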(event `self.ReceiveBeginPlay`
  ;[1 1 1] Set player ref + bind to pickup delegate
  (`parent.ReceiveBeginPlay`)
  (bind _asbp_player_character (cast `/Game/Blueprints/PlayerCharacter/BP_PlayerCharacter` (`A_BlueprintFunctionLibrary.GetActivePlayerCharacter`)))
  (bind _output_get (set `self.PlayerRef` _asbp_player_character))
  (add `/Game/Blueprints/PlayerCharacter/BP_PlayerCharacter.Pickup_Event` _output_get (delegate `Pickup_Sequence`)))

(event `Pickup_Sequence`
  ;[1 1 1] Pickup Sequence Event
  (if (`self.bInteractable`)
    (`/Game/Blueprints/PlayerCharacter/BP_PlayerCharacter.SetTreasureCountStats` (`self.PlayerRef`) (`self.ScoreVale`))
    (`self.K2_DestroyActor`)))

(fn `UserConstructionScript`
  (`parent.UserConstructionScript`)
  (set `self.ScoreVale` 15))